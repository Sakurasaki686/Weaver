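; Interactable chest Blueprint that costs Aether to open and offers the player a choice of affix rewards.
; BeginPlay builds the hint text from the cost.
; Open plays the chest montage, immediately deducts Aether through a SetByCaller gameplay effect, and has RewardComponent start reward selection on the "OpenFinished" notify.
; The StartRewardSelection event creates the affix selection widget and broadcasts three random unique affixes through the player's UI component.
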(event EventBeginPlay
  (Variables|Default|SetChestInteractionHint (Utilities|Text|FormatText "Cost Aether: {AetherAmount}" (Variables|Default|GetAetherCostToOpen))))

(event Collision|EventActorBeginOverlap
  (params (OtherActor :type Actor%20Object%20Reference)))

(event EventTick
  (params (DeltaSeconds :type Float%20%28single-precision%29)))

(event EventOpen
  (params (InInstigator :type Actor%20Object%20Reference))
  (Variables|Default|SetIn%20Instigator InInstigator)
  (bind _notifyname (Animation|Montage|PlayMontage (Variables|Default|GetChestMesh) (.AsAnim%20Montage (Utilities|Casting|CastToAnimMontage (Variables|Default|GetOpenAnimation))))
    (:then
      (bind _asweaver_player_character (Utilities|Casting|CastToWeaverPlayerCharacter (Variables|Default|GetIn%20Instigator)))
      (bind _returnvalue (Ability|GameplayEffect|AssignTagSetbyCallerMagnitude (GameplayEffects|MakeOutgoingSpec :self (Variables|/Script/Weaver.WeaverBaseCharacter|GetWeaverAbilitySystemComponent _asweaver_player_character) :GameplayEffectClass "/Game/Shared/GameplayEffects/GE_Shared_ChangePlayerAetherAmount.GE_Shared_ChangePlayerAetherAmount_C") "(TagName=\"Shared.SetByCaller.AetherChangeAmount\")" (* (Variables|Default|GetAetherCostToOpen) -1.0)))
      (GameplayEffects|ApplyGameplayEffectSpecToSelf (Variables|/Script/Weaver.WeaverBaseCharacter|GetWeaverAbilitySystemComponent _asweaver_player_character) _returnvalue))
    (:OnNotifyBegin
      (if (== _notifyname "OpenFinished")
        (Class|WeaverRewardComponent|StartRewardSelection (Variables|Default|GetRewardComponent))))))

(event EventStartRewardSelection
  (bind _asweaver_player_controller (Utilities|Casting|CastToWeaverPlayerController (Game|GetInstigatorController (Variables|Default|GetIn%20Instigator))))
  (bind _returnvalue (UserInterface|CreateWidget "/Game/Widgets/AffixesWidgets/WBP_AffixesSelectWidget.WBP_AffixesSelectWidget_C" _asweaver_player_controller))
  (UserInterface|Viewport|AddtoViewport _returnvalue 0)
  (bind _asweaver_player_character (Utilities|Casting|CastToWeaverPlayerCharacter (Variables|Default|GetIn%20Instigator)))
  (Class|PlayerUIComponent|BroadcastChestOpened (Variables|/Script/Weaver.WeaverPlayerCharacter|GetPlayerUIComponent _asweaver_player_character) (Class|WeaverRewardComponent|GetRandomUniqueAffixes (Variables|Default|GetRewardComponent) 3)))

(fn ConstructionScript)