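; Projectile Blueprint for Sevarog's slash, with almost all behavior left outside this graph.
; Its SetupCollision function makes the collision box ignore the instigator while moving, assigns it a custom trace channel as object type and ignores another custom channel.
; The construction script only calls the parent, and the event graph holds no active logic.
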(event EventBeginPlay
  (|CallParentFunction) ; This node is disabled and will not be called.\nDrag off pins to build functionality.
)

(event Collision|EventActorBeginOverlap
  (params (OtherActor :type Actor%20Object%20Reference)))

(event EventTick
  (params (DeltaSeconds :type Float%20%28single-precision%29)))

(fn ConstructionScript
  (|CallParentFunction))

(fn SetupCollision
  (Collision|IgnoreActorwhenMoving (Variables|Default|GetProjectileCollisionBox) (Variables|Default|GetInstigator) true)
  (Collision|SetCollisionObjectType (Variables|Default|GetProjectileCollisionBox) "ECC_GameTraceChannel4")
  (Collision|SetCollisionResponsetoChannel (Variables|Default|GetProjectileCollisionBox) "ECC_GameTraceChannel3" "ECR_Ignore"))