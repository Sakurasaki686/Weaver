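; Interactable gambling mushroom that gives the interacting player a random punishment, reward or special reward, then recharges after a cooldown.
; An attached Niagara hint doubles as the availability flag: the box overlap prompt and Interact require it, and a timer respawns it.
; A roll from GambleEventsPool selects a gameplay tag that applies a GAS effect, with hit react on punishment, or grants a random affix.
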(event OnComponentBeginOverlap(Box)
  (params (OverlappedComponent :type Primitive%20Component%20Object%20Reference) (OtherActor :type Actor%20Object%20Reference) (OtherComp :type Primitive%20Component%20Object%20Reference) (OtherBodyIndex :type Integer) (bFromSweep :type Boolean) (SweepResult :type Hit%20Result%20Structure%20%28by%20ref%29))
  (Variables|Default|GetInteractableHint
    (:then
      (Class|PawnInteractionInterface|SetInteractionInfo(Message) OtherActor self (Variables|Default|GetIn%20Interaction%20Prompt)))
    (:else)))

(event OnComponentEndOverlap(Box)
  (params (OverlappedComponent :type Primitive%20Component%20Object%20Reference) (OtherActor :type Actor%20Object%20Reference) (OtherComp :type Primitive%20Component%20Object%20Reference) (OtherBodyIndex :type Integer))
  (Class|PawnInteractionInterface|SetInteractionInfo(Message) OtherActor 0 (Variables|Default|GetIn%20Interaction%20Prompt)))

(event Custom|ResetState
  (CallFunction|InitializeNewInteracableHint))

(event EventBeginPlay
  (CallFunction|InitializeNewInteracableHint))

(event EventInteract
  (params (InInstigator :type Actor%20Object%20Reference))
  (bind _interactablehint (Variables|Default|GetInteractableHint)
    (:then
      (Components|DestroyComponent _interactablehint)
      (Components|Activation|Activate (Variables|Default|GetInteractionFeedbackEffect%20) false)
      (Class|PawnInteractionInterface|SetInteractionInfo(Message) InInstigator 0 (Variables|Default|GetIn%20Interaction%20Prompt))
      (Audio|SpawnSoundatLocation "/Game/Magic___Spell_Sounds_PRO/General/cue/Buff_Attack_9_1_Cue.Buff_Attack_9_1_Cue" (Transformation|GetActorLocation) "0, 0, 0" 1.0 1.0 0.0 0 0)
      (CallFunction|HandleGambleResult InInstigator)
      (Utilities|Time|SetTimerbyEvent (delegate Custom|ResetState) (Variables|Default|GetGambleCooldown)))
    (:else)))

(fn ConstructionScript)

(fn InitializeNewInteracableHint
  (bind _returnvalue (Niagara|SpawnSystemAttached "/Game/Projectiles_Spells_VFX_Vol_2/Effects/GreenHalo/Lvl_3/NS_Projectile_25_Lvl_3.NS_Projectile_25_Lvl_3" (Variables|Default|GetInteractableHintSocket) "None" "0, 0, 0" "0, 0, 0" "KeepRelativeOffset" false))
  (Variables|Default|SetInteractableHint _returnvalue))

(fn HandleGambleResult
  (params (InInstigator :type Actor%20Object%20Reference))
  (bind _gambleeventspool (Variables|Default|GetGambleEventsPool))
  (bind (_outselectedeventtag _returnvalue) (Class|WeaverFunctionLibrary|SelectRandomGambleEvent _gambleeventspool))
  (bind _asweaver_player_character (Utilities|Casting|CastToWeaverPlayerCharacter InInstigator))
  (LocalVariables|SetPlayerCharacter _asweaver_player_character)
  (if _returnvalue
    (|SwitchGameplayTag _outselectedeventtag
      (:Interactable.Mushroom.Event.Punishment
        (GameplayEffects|ApplyGameplayEffectSpecToTarget (Variables|/Script/Weaver.WeaverBaseCharacter|GetWeaverAbilitySystemComponent (LocalVariables|GetPlayerCharacter)) (GameplayEffects|MakeOutgoingSpec :self (Variables|/Script/Weaver.WeaverBaseCharacter|GetWeaverAbilitySystemComponent (LocalVariables|GetPlayerCharacter)) :GameplayEffectClass "/Game/Shared/Mushroom/GameplayEffects/GE_Mushroom_Punishment.GE_Mushroom_Punishment_C" :Level 1.0) (Variables|/Script/Weaver.WeaverBaseCharacter|GetWeaverAbilitySystemComponent (LocalVariables|GetPlayerCharacter)))
        (Ability|SendGameplayEventtoActor (LocalVariables|GetPlayerCharacter) "(TagName=\"Shared.Event.HitReact\")" (Utilities|Struct|MakeGameplayEventData "(TagName=\"\")" self)))
      (:Interactable.Mushroom.Event.Reward
        (GameplayEffects|ApplyGameplayEffectSpecToTarget (Variables|/Script/Weaver.WeaverBaseCharacter|GetWeaverAbilitySystemComponent (LocalVariables|GetPlayerCharacter)) (GameplayEffects|MakeOutgoingSpec :self (Variables|/Script/Weaver.WeaverBaseCharacter|GetWeaverAbilitySystemComponent (LocalVariables|GetPlayerCharacter)) :GameplayEffectClass "/Game/Shared/Mushroom/GameplayEffects/GE_Mushroom_Reward.GE_Mushroom_Reward_C" :Level 1.0) (Variables|/Script/Weaver.WeaverBaseCharacter|GetWeaverAbilitySystemComponent (LocalVariables|GetPlayerCharacter))))
      (:Interactable.Mushroom.Event.SpecialReward
        (bind _output_get (LocalVariables|SetRolledAffix (Utilities|Array|Get(acopy) (Class|WeaverRewardComponent|GetRandomUniqueAffixes (Variables|Default|GetWeaverReward) 1))))
        (Class|PlayerCombatComponent|AddAffix (Variables|/Script/Weaver.WeaverPlayerCharacter|GetPlayerCombatComponent (LocalVariables|GetPlayerCharacter)) _output_get)
        (Class|PawnInteractionInterface|ShowInteractionHintFeedback (LocalVariables|GetPlayerCharacter) (Utilities|Text|ToText(String) (Utilities|String|Append "Acquire New Affix: " (Utilities|String|ToString(Text) (Variables|/Script/Weaver.DataAsset_AffixBase|GetDisplayName _output_get)) "!")))))))