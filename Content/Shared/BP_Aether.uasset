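; BP_Aether is an Aether pickup that grants the player Aether on touch.
; Overlapping its interaction box with a WeaverPlayerCharacter applies a GAS effect spec to that player, passing the change amount via a SetByCaller tag.
; It then plays a pickup sound and destroys itself.
; An attached looping sound fades in on BeginPlay, and on destruction gets a fade-out call followed immediately by component destruction.
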(event EventBeginPlay
  (bind _returnvalue (Audio|SpawnSoundAttached (Variables|Default|GetLoopingSound) (Variables|Transformation|GetRootComponent) "None" "0, 0, 0" "0, 0, 0" "KeepRelativeOffset" false 1.0 1.0 0.0 0 0))
  (bind _output_get (Variables|Default|SetLoopingSoundComponent _returnvalue))
  (Audio|Components|Audio|FadeIn _output_get 1.0 1.0 0.0 "Linear" :!class /Script/Engine.AudioComponent))

(event Collision|EventActorBeginOverlap
  (params (OtherActor :type Actor%20Object%20Reference)))

(event EventTick
  (params (DeltaSeconds :type Float%20%28single-precision%29)))

(event EventDestroyed
  (bind _loopingsoundcomponent (Variables|Default|GetLoopingSoundComponent))
  (Audio|Components|Audio|FadeOut _loopingsoundcomponent 1.0 0.0 "Linear" :!class /Script/Engine.AudioComponent)
  (Components|DestroyComponent _loopingsoundcomponent))

(event EventOnInteractionBoxBeginOverlap
  (params (OverlappedComponent :type Primitive%20Component%20Object%20Reference) (OtherActor :type Actor%20Object%20Reference) (OtherComp :type Primitive%20Component%20Object%20Reference) (OtherBodyIndex :type Integer) (bFromSweep :type Boolean) (SweepResult :type Hit%20Result%20Structure%20%28by%20ref%29))
  (bind _asweaver_player_character (Utilities|Casting|CastToWeaverPlayerCharacter OtherActor))
  (bind _returnvalue (Ability|GameplayEffect|AssignTagSetbyCallerMagnitude (GameplayEffects|MakeOutgoingSpec :self (Variables|/Script/Weaver.WeaverBaseCharacter|GetWeaverAbilitySystemComponent _asweaver_player_character) :GameplayEffectClass "/Game/Shared/GameplayEffects/GE_Shared_ChangePlayerAetherAmount.GE_Shared_ChangePlayerAetherAmount_C") "(TagName=\"Shared.SetByCaller.AetherChangeAmount\")" 1.0))
  (GameplayEffects|ApplyGameplayEffectSpecToSelf (Variables|/Script/Weaver.WeaverBaseCharacter|GetWeaverAbilitySystemComponent _asweaver_player_character) _returnvalue)
  (Audio|PlaySoundatLocation (Variables|Default|GetPickupSound) (Transformation|GetActorLocation) "0, 0, 0" 1.0 1.0 0.0 0 0 0 0)
  (Actor|DestroyActor))

(fn ConstructionScript)