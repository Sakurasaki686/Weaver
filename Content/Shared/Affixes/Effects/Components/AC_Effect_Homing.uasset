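; Affix effect component that turns its owning projectile into a homing projectile when initialized.
; For player-fired projectiles, a wide box trace from the player along the follow camera's forward vector picks the first hit actor's root as the homing target.
; For enemy-fired projectiles, the target comes from the enemy's TargetActor blackboard key.
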(event EventBeginPlay)

(event EventTick
  (params (DeltaSeconds :type Float%20%28single-precision%29)))

(event EventInitializeComponentforProjectile
  (bind _returnvalue (Components|GetOwner))
  (bind _owningprojectile (Variables|Default|GetOwningProjectile))
  (bind _projectilemovementcomp (Variables|/Script/Weaver.WeaverProjectileBase|GetProjectileMovementComp _owningprojectile))
  (bind _instigator (Variables|/Script/Engine.Actor|GetInstigator _returnvalue))
  (Variables|/Script/Engine.ProjectileMovementComponent|SetbIsHomingProjectile _projectilemovementcomp true)
  (bind _asweaver_player_character (Utilities|Casting|CastToWeaverPlayerCharacter _instigator)
    (:then
      (CallFunction|HandlePlayerProjectileHoming _projectilemovementcomp _asweaver_player_character))
    (:CastFailed
      (bind _asweaver_enemy_character (Utilities|Casting|CastToWeaverEnemyCharacter _instigator))
      (CallFunction|HandleEnemyProjectileHoming _projectilemovementcomp _asweaver_enemy_character))))

(fn HandlePlayerProjectileHoming
  (params (ProjectileMovementComp :type Projectile%20Movement%20Component%20Object%20Reference) (PlayerCharacter :type Weaver%20Player%20Character%20Object%20Reference))
  (bind _actors_to_ignore (Variables|Default|GetActors%20to%20Ignore))
  (bind _returnvalue (Transformation|GetActorLocation PlayerCharacter))
  (Utilities|Array|Add _actors_to_ignore PlayerCharacter)
  (bind (_outhit _returnvalue_2) (Class|KismetSystemLibrary|BoxTraceSingleforObjects _returnvalue (+ _returnvalue (* 3e+03 (Math|Vector|GetForwardVector (Variables|/Script/Weaver.WeaverPlayerCharacter|GetFollowCamera PlayerCharacter)))) "500.000000,1500.000000,500.000000" "0, 0, 0" (Variables|Default|GetObject%20Types) false _actors_to_ignore "None" true "(R=1.000000,G=0.000000,B=0.000000,A=1.000000)" "(R=0.000000,G=1.000000,B=0.000000,A=1.000000)" 2.0))
  (if _returnvalue_2
    (Variables|/Script/Engine.ProjectileMovementComponent|SetHomingTargetComponent ProjectileMovementComp (Variables|/Script/Engine.Actor|GetRootComponent (.HitActor (Collision|BreakHitResult _outhit))))))

(fn HandleEnemyProjectileHoming
  (params (ProjectileMovementComp :type Projectile%20Movement%20Component%20Object%20Reference) (EnemyCharacter :type Weaver%20Enemy%20Character%20Object%20Reference))
  (bind _asactor (Utilities|Casting|CastToActor (AI|Components|Blackboard|GetValueasObject (AI|GetBlackboard EnemyCharacter) (Utilities|Name|MakeLiteralName "TargetActor"))))
  (Variables|/Script/Engine.ProjectileMovementComponent|SetHomingTargetComponent ProjectileMovementComp (Variables|/Script/Engine.Actor|GetRootComponent _asactor)))