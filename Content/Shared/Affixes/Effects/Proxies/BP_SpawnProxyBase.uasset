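; Base spawn proxy for affix effects that launches element projectiles from a Weaver character.
; ExecuteSpawn stores the instigator, tuner tag, and element and effect data assets, then caches the mesh's ProjectileSocket location and forward vector.
; A separate event spawns the element's projectile class there with a given rotation, then attaches and initializes the effect's component.
; ExecuteSpawn itself spawns nothing.
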(event Custom|SpawnProjectileAndInitializeAtSocketLocation
  (params (Spawn%20Transform%20Rotation :type Rotator))
  (bind _returnvalue (Game|SpawnActorfromClass :Class (Variables|/Script/Weaver.DataAsset_ElementBase|GetProjectileClass (Variables|Default|GetIn%20Element%20DA)) :SpawnTransform (Math|Transform|MakeTransform (Variables|Default|GetProjectileSocketLocation) Spawn%20Transform%20Rotation "1.000000,1.000000,1.000000") :CollisionHandlingOverride "AlwaysSpawn" :TransformScaleMethod "MultiplyWithRoot" :Instigator (Variables|Default|GetInstigatorCharacter)))
  (bind _returnvalue_2 (Game|AddComponentbyClass _returnvalue (Variables|/Script/Weaver.DataAsset_EffectBase|GetEffectComponentClass (Variables|Default|GetIn%20Effect%20DA))))
  (Class|ProjectileExtensionComponentBase|InitializeComponentforProjectile _returnvalue_2))

(event EventBeginPlay)

(event Collision|EventActorBeginOverlap
  (params (OtherActor :type Actor%20Object%20Reference)))

(event EventTick
  (params (DeltaSeconds :type Float%20%28single-precision%29)))

(event EventExecuteSpawn
  (params (InInstigator :type Actor%20Object%20Reference) (InTunerTag :type Gameplay%20Tag%20Structure%20%28by%20ref%29) (InElementDA :type Data%20Asset%20Element%20Base%20Object%20Reference) (InEffectDA :type Data%20Asset%20Effect%20Base%20Object%20Reference))
  (bind _asweaver_base_character (Utilities|Casting|CastToWeaverBaseCharacter InInstigator))
  (Variables|Default|SetInstigatorCharacter _asweaver_base_character)
  (Variables|Default|SetIn%20Tuner%20Tag InTunerTag)
  (Variables|Default|SetIn%20Element%20DA InElementDA)
  (Variables|Default|SetIn%20Effect%20DA InEffectDA)
  (Variables|Default|SetProjectileSocketLocation (.location (Transformation|GetSocketTransform (Variables|/Script/Engine.Character|GetMesh (Variables|Default|GetInstigatorCharacter)) "ProjectileSocket" "RTS_World")))
  (Variables|Default|SetProjectileSocketForwardVector (Math|Vector|GetForwardVector (.rotation (Transformation|GetSocketTransform (Variables|/Script/Engine.Character|GetMesh (Variables|Default|GetInstigatorCharacter)) "ProjectileSocket" "RTS_World")))))

(fn ConstructionScript)