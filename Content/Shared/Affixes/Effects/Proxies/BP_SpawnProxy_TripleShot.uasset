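; Spawn proxy for the TripleShot affix effect that fires several projectiles toward the player's camera aim when ExecuteSpawn runs.
; After the parent call, it line-traces from the follow camera and chooses a rotation from the hit, or the trace end on a miss.
; It spawns NumberOfShots element-defined projectiles at the socket, each receiving the effect's component.
; All shots share the same location and aim, with no spread applied.
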(event EventBeginPlay)

(event Collision|EventActorBeginOverlap
  (params (OtherActor :type Actor%20Object%20Reference)))

(event EventTick
  (params (DeltaSeconds :type Float%20%28single-precision%29)))

(event EventExecuteSpawn
  (params (InInstigator :type Actor%20Object%20Reference) (InTunerTag :type Gameplay%20Tag%20Structure%20%28by%20ref%29) (InElementDA :type Data%20Asset%20Element%20Base%20Object%20Reference) (InEffectDA :type Data%20Asset%20Effect%20Base%20Object%20Reference))
  (bind _playercharacter (Variables|Default|GetPlayerCharacter))
  (bind _followcamera (Variables|/Script/Weaver.WeaverPlayerCharacter|GetFollowCamera _playercharacter))
  (bind _returnvalue (Transformation|GetWorldLocation _followcamera))
  (|CallParentFunction InInstigator InTunerTag InElementDA InEffectDA)
  (bind _output_get (Variables|Default|SetCameraForwardVector (Math|Vector|GetForwardVector (Transformation|GetWorldRotation _followcamera))))
  (bind (_outhit _returnvalue_2) (Collision|LineTraceForObjects _returnvalue (+ (* _output_get (Variables|Default|GetMaxTraceDistance)) _returnvalue) (Variables|Default|GetObject%20Type) false 0 "None"))
  (for _index (range 0 (- (Variables|Default|GetNumberOfShots) 1))
    (bind _returnvalue_3 (Game|SpawnActorfromClass :Class (Variables|/Script/Weaver.DataAsset_ElementBase|GetProjectileClass (Variables|Default|GetIn%20Element%20DA)) :SpawnTransform (Math|Transform|MakeTransform (Variables|Default|GetProjectileSocketLocation) (Math|Rotator|SelectRotator (Math|Rotator|FindLookatRotation (Variables|Default|GetProjectileSocketLocation) (.Location (Collision|BreakHitResult _outhit))) (Math|Rotator|FindLookatRotation (.Location (Collision|BreakHitResult _outhit)) (+ (* _output_get (Variables|Default|GetMaxTraceDistance)) _returnvalue)) _returnvalue_2) "1.000000,1.000000,1.000000") :CollisionHandlingOverride "AdjustIfPossibleButAlwaysSpawn" :TransformScaleMethod "MultiplyWithRoot" :Instigator (Variables|Default|GetPlayerCharacter)))
    (bind _returnvalue_4 (Game|AddComponentbyClass _returnvalue_3 (Variables|/Script/Weaver.DataAsset_EffectBase|GetEffectComponentClass (Variables|Default|GetIn%20Effect%20DA))))
    (Class|ProjectileExtensionComponentBase|InitializeComponentforProjectile _returnvalue_4)))

(fn ConstructionScript)