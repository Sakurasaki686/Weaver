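; Spawn proxy for a multi-shot affix effect that fires several projectiles from the instigator's projectile socket in an evenly spaced fan.
; Players aim via a follow-camera trace, falling back to the trace's far point when nothing is hit or the hit lies behind the socket.
; Enemies aim at their blackboard TargetActor.
; CalculateMultiShotRot spreads that aim across SpreadAngle around the camera's or target's up axis, spawning one projectile per rotation.
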(event EventBeginPlay)

(event Collision|EventActorBeginOverlap
  (params (OtherActor :type Actor%20Object%20Reference)))

(event EventTick
  (params (DeltaSeconds :type Float%20%28single-precision%29)))

(event EventExecuteSpawn
  (params (InInstigator :type Actor%20Object%20Reference) (InTunerTag :type Gameplay%20Tag%20Structure%20%28by%20ref%29) (InElementDA :type Data%20Asset%20Element%20Base%20Object%20Reference) (InEffectDA :type Data%20Asset%20Effect%20Base%20Object%20Reference))
  (|CallParentFunction InInstigator InTunerTag InElementDA InEffectDA)
  (Utilities|FlowControl|Sequence
    (:then_0
      (bind _asweaver_player_character (Utilities|Casting|CastToWeaverPlayerCharacter (Variables|Default|GetInstigatorCharacter)))
      (bind _output_get (Variables|Calculation|SetCameraForwardVector (Math|Vector|GetForwardVector (Transformation|GetWorldRotation (Variables|/Script/Weaver.WeaverPlayerCharacter|GetFollowCamera _asweaver_player_character)))))
      (Variables|Calculation|SetCameraUpVector (Math|Vector|GetUpVector (Transformation|GetWorldRotation (Variables|/Script/Weaver.WeaverPlayerCharacter|GetFollowCamera _asweaver_player_character))))
      (bind (_outhit _returnvalue) (Collision|LineTraceForObjects (Transformation|GetWorldLocation (Variables|/Script/Weaver.WeaverPlayerCharacter|GetFollowCamera _asweaver_player_character)) (+ (* _output_get (Variables|Default|GetMaxTraceDistance)) (Transformation|GetWorldLocation (Variables|/Script/Weaver.WeaverPlayerCharacter|GetFollowCamera _asweaver_player_character))) (Variables|Default|GetObject%20Type) false 0 "None"))
      (bind _outrots (CallFunction|CalculateMultiShotRot (Math|Vector|GetForwardVector (Math|Rotator|SelectRotator (Math|Rotator|MakeRotfromX (- (+ (* _output_get (Variables|Default|GetMaxTraceDistance)) (Transformation|GetWorldLocation (Variables|/Script/Weaver.WeaverPlayerCharacter|GetFollowCamera _asweaver_player_character))) (Variables|Default|GetProjectileSocketLocation))) (Math|Rotator|FindLookatRotation (Variables|Default|GetProjectileSocketLocation) (.Location (Collision|BreakHitResult _outhit))) (or (not _returnvalue) (<= (Math|Vector|DotProduct (Variables|Default|GetProjectileSocketForwardVector) (- (.ImpactPoint (Collision|BreakHitResult _outhit)) (Variables|Default|GetProjectileSocketLocation))) 0.0)))) (Variables|Calculation|GetCameraUpVector)))
      (for _array_element _outrots
        (CallFunction|SpawnProjectileandInitializeatSocketLocation _array_element)))
    (:then_1
      (bind _asweaver_enemy_character (Utilities|Casting|CastToWeaverEnemyCharacter (Variables|Default|GetInstigatorCharacter)))
      (bind _asactor (Utilities|Casting|CastToActor (AI|Components|Blackboard|GetValueasObject (AI|GetBlackboard _asweaver_enemy_character) (Utilities|Name|MakeLiteralName "TargetActor"))))
      (bind _outrots_2 (CallFunction|CalculateMultiShotRot (- (Transformation|GetActorLocation _asactor) (Variables|Default|GetProjectileSocketLocation)) (Transformation|GetActorUpVector _asactor)))
      (for _array_element_2 _outrots_2
        (CallFunction|SpawnProjectileandInitializeatSocketLocation _array_element_2)))))

(fn ConstructionScript)

(fn CalculateMultiShotRot
  (params (BaseAimDirection :type Vector) (AxisToRotateAround :type Vector))
  (LocalVariables|SetAngleStep (/ (Variables|MultiShotControls|GetSpreadAngle) (- (Variables|MultiShotControls|GetNumberOfShots) 1)))
  (LocalVariables|SetStartAngle (/ (Variables|MultiShotControls|GetSpreadAngle) -2.0))
  (for _index (range 0 (- (Variables|MultiShotControls|GetNumberOfShots) 1))
    (Utilities|Array|Add (LocalVariables|GetOutRotArray) (Math|Conversions|RotationFromXVector (Math|Vector|RotateVectorAroundAxis BaseAimDirection (+ (LocalVariables|GetStartAngle) (* _index (LocalVariables|GetAngleStep))) AxisToRotateAround))))
  (return (LocalVariables|GetOutRotArray)))