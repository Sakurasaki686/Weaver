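; BP_BGMManager is a background music manager that plays music through an AudioComponent with timed fade-ins.
; On BeginPlay it fades the component in and binds OnAudioFinished to fade it in again, so the music restarts whenever playback finishes.
; SetupSound changes the track and volume multiplier, calling fade out, the swap and fade in back to back with no wait between them.
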(event Custom|OnAudioFinished_Event
  (Audio|Components|Audio|FadeIn (Variables|Default|GetAudioComponent) 5.0 1.0 0.0 "Linear" :!class /Script/Engine.AudioComponent))

(event EventBeginPlay
  (bind _audiocomponent (Variables|Default|GetAudioComponent))
  (Audio|Components|Audio|FadeIn _audiocomponent 5.0 1.0 0.0 "Linear" :!class /Script/Engine.AudioComponent)
  (EventDispatchers|AssignOnAudioFinished _audiocomponent (delegate Custom|OnAudioFinished_Event)))

(fn ConstructionScript
  (|CallParentFunction))

(fn SetupSound
  (params (NewSound :type Sound%20Base%20Object%20Reference) (Volume%20Multiplier :type Float%20%28double-precision%29))
  (bind _audiocomponent (Variables|Default|GetAudioComponent))
  (Audio|Components|Audio|FadeOut _audiocomponent 5.0 0.0 "Linear" :!class /Script/Engine.AudioComponent)
  (Audio|Components|Audio|SetSound _audiocomponent NewSound)
  (Audio|Components|Audio|SetVolumeMultiplier _audiocomponent Volume%20Multiplier :!class /Script/Engine.AudioComponent)
  (Audio|Components|Audio|FadeIn _audiocomponent 5.0 1.0 0.0 "Linear" :!class /Script/Engine.AudioComponent))