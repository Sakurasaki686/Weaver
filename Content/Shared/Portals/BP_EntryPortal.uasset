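; Entry portal actor that moves any actor overlapping its trigger volume to a newly spawned exit portal.
; On overlap it spawns BP_ExitPortal at the first actor tagged ExitPortalSpawnPoint, relocates the overlapping actor there and plays a spell sound at the entry.
; When the overlap ends it deactivates the Portal component and fades out two cached portal sounds.
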(event Custom|OnComponentBeginOverlap_Event
  (params (OverlappedComponent :type Primitive%20Component%20Object%20Reference) (OtherActor :type Actor%20Object%20Reference) (OtherComp :type Primitive%20Component%20Object%20Reference) (OtherBodyIndex :type Integer) (bFromSweep :type Boolean) (SweepResult :type Hit%20Result%20Structure%20%28by%20ref%29))
  (Utilities|FlowControl|Sequence
    (:then_0
      (bind _outactors (Actor|GetAllActorswithTag "ExitPortalSpawnPoint"))
      (bind _returnvalue (Game|SpawnActorfromClass "/Game/Shared/Portals/BP_ExitPortal.BP_ExitPortal_C" (Math|Transform|MakeTransform (.location (Transformation|GetActorTransform (Utilities|Array|Get(acopy) _outactors))) (Math|Rotator|MakeRotator (.roll (.rotation (Transformation|GetActorTransform (Utilities|Array|Get(acopy) _outactors)))) 0.0 (.yaw (.rotation (Transformation|GetActorTransform (Utilities|Array|Get(acopy) _outactors))))) "1.000000,1.000000,1.000000") "AdjustIfPossibleButAlwaysSpawn" "MultiplyWithRoot" 0 0))
      (Transformation|SetActorLocation OtherActor (Transformation|GetActorLocation _returnvalue) false false))
    (:then_1
      (Audio|PlaySoundatLocation "/Game/Magic___Spell_Sounds_PRO/Elements___School/Arcane/cue/Arcane_Spell_13_2_Cue.Arcane_Spell_13_2_Cue" (Transformation|GetActorLocation) "0, 0, 0" 1.5 1.0 0.0 0 0 0 0))))

(event Custom|OnComponentEndOverlap_Event
  (params (OverlappedComponent :type Primitive%20Component%20Object%20Reference) (OtherActor :type Actor%20Object%20Reference) (OtherComp :type Primitive%20Component%20Object%20Reference) (OtherBodyIndex :type Integer))
  (Components|Activation|Deactivate (Variables|Default|GetPortal))
  (Audio|Components|Audio|FadeOut (Variables|Default|GetCachedPortalSound_1) 2.0 0.0 "Linear" :!class /Script/Engine.AudioComponent)
  (Audio|Components|Audio|FadeOut (Variables|Default|GetCachedPortalSound_2) 2.0 0.0 "Linear" :!class /Script/Engine.AudioComponent))

(event EventBeginPlay
  (|CallParentFunction)
  (Collision|AssignOnComponentBeginOverlap (Variables|Default|GetTriggerVolume) (EventDispatchers|CreateEvent :!event Custom|OnComponentBeginOverlap_Event))
  (Collision|AssignOnComponentEndOverlap (Variables|Default|GetTriggerVolume) (EventDispatchers|CreateEvent :!event Custom|OnComponentEndOverlap_Event)))

(fn ConstructionScript)