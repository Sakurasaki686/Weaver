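; BP_ExitPortal is an exit portal that shuts down its effect and sound shortly after something overlaps its trigger volume.
; BeginPlay runs the parent logic, then binds the trigger's begin-overlap event, which does not filter the overlapping actor.
; After a brief delay, the overlap deactivates Portal and fades out two cached sounds, the second only if the first is valid.
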(event Custom|OnComponentBeginOverlap_Event
  (params (OverlappedComponent :type Primitive%20Component%20Object%20Reference) (OtherActor :type Actor%20Object%20Reference) (OtherComp :type Primitive%20Component%20Object%20Reference) (OtherBodyIndex :type Integer) (bFromSweep :type Boolean) (SweepResult :type Hit%20Result%20Structure%20%28by%20ref%29))
  (bind _cachedportalsound_1 (Variables|Default|GetCachedPortalSound_1))
  (bind _cachedportalsound_2 (Variables|Default|GetCachedPortalSound_2))
  (Utilities|FlowControl|Delay 1.0)
  (Components|Activation|Deactivate (Variables|Default|GetPortal))
  (Utilities|IsValid _cachedportalsound_1
    (:Is%20Valid
      (Audio|Components|Audio|FadeOut _cachedportalsound_1 2.0 0.0 "Linear" :!class /Script/Engine.AudioComponent)
      (Utilities|IsValid _cachedportalsound_2
        (:Is%20Valid
          (Audio|Components|Audio|FadeOut _cachedportalsound_2 2.0 0.0 "Linear" :!class /Script/Engine.AudioComponent))))))

(event EventBeginPlay
  (|CallParentFunction)
  (Collision|AssignOnComponentBeginOverlap (Variables|Default|GetTriggerVolume) (EventDispatchers|CreateEvent :!event Custom|OnComponentBeginOverlap_Event)))

(event Collision|EventActorBeginOverlap
  (params (OtherActor :type Actor%20Object%20Reference)))

(event EventTick
  (params (DeltaSeconds :type Float%20%28single-precision%29)))

(fn ConstructionScript)