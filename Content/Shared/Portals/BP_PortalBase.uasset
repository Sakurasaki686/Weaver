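; BP_PortalBase is a portal actor that pairs a particle effect with looping ambient audio.
; On BeginPlay it spawns two looping sounds attached to the root, caches both and fades them in.
; It also binds to the Portal system's finished event, so the actor destroys itself when the effect completes.
; Overlap, tick and construction logic are empty.
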(event Custom|OnSystemFinished_Event
  (params (PSystem :type Niagara%20Component%20Object%20Reference))
  (Actor|DestroyActor))

(event EventBeginPlay
  (Utilities|FlowControl|Sequence
    (:then_0
      (bind _returnvalue (Audio|SpawnSoundAttached "/Game/Magic___Spell_Sounds_PRO/Casting___Loops/cue/Field_2_Loop_Cue.Field_2_Loop_Cue" (Variables|Transformation|GetRootComponent) "None" "0, 0, 0" "0, 0, 0" "KeepRelativeOffset" false 3.0 1.0 0.0 0 0))
      (bind _output_get (Variables|Default|SetCachedPortalSound_1 _returnvalue))
      (Audio|Components|Audio|FadeIn _output_get 2.0 1.0 0.0 "Linear" :!class /Script/Engine.AudioComponent)
      (bind _returnvalue_2 (Audio|SpawnSoundAttached "/Game/Magic___Spell_Sounds_PRO/Casting___Loops/cue/Holy_Cast_Loop_1_Cue.Holy_Cast_Loop_1_Cue" (Variables|Transformation|GetRootComponent) "None" "0, 0, 0" "0, 0, 0" "KeepRelativeOffset" false 1.0 1.0 0.0 0 0))
      (bind _output_get_2 (Variables|Default|SetCachedPortalSound_2 _returnvalue_2))
      (Audio|Components|Audio|FadeIn _output_get_2 2.0 1.0 0.0 "Linear" :!class /Script/Engine.AudioComponent))
    (:then_1
      (EventDispatchers|AssignOnSystemFinished (Variables|Default|GetPortal) (EventDispatchers|CreateEvent :!event Custom|OnSystemFinished_Event)))))

(event Collision|EventActorBeginOverlap
  (params (OtherActor :type Actor%20Object%20Reference)))

(event EventTick
  (params (DeltaSeconds :type Float%20%28single-precision%29)))

(fn ConstructionScript)