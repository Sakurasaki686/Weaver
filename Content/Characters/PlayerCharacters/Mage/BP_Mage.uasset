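; BP_Mage is the Mage player character, which sets up its starting combat loadout and handles dig input.
; On BeginPlay it gives the combat component a Focus tuner, Arcane element and Empty effect.
; It also self-applies a GAS effect that receives the Focus attack multiplier through a SetByCaller tag.
; The Dig input holds a sculpt-mode gameplay tag on the character until released or canceled.
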(event Input|EnhancedActionEvents|EnhancedInputActionIA_Dig
  (params (ActionValue :type Boolean) (ElapsedSeconds :type Float%20%28double-precision%29) (TriggeredSeconds :type Float%20%28double-precision%29) (InputAction :type Input%20Action%20Object%20Reference :default "/Game/Characters/PlayerCharacters/Mage/Input/Actions/IA_Dig.IA_Dig"))
  (:Started
    (Class|WeaverFunctionLibrary|AddGameplayTagtoActorifNone self "(TagName=\"Player.SculptMode.Dig\")"))
  (:Canceled
    (Class|WeaverFunctionLibrary|RemoveGameplayTagfromActorifFound self "(TagName=\"Player.SculptMode.Dig\")" :!label _label))
  (:Completed
    (goto _label)))

(event EventBeginPlay
  (Utilities|FlowControl|Sequence
    (:then_0
      (Class|PlayerCombatComponent|AddandSetTuner (Variables|Default|GetPlayerCombatComponent) "/Game/Shared/Affixes/Tuners/DA_Tuner_Focus.DA_Tuner_Focus")
      (bind _returnvalue (Ability|GameplayEffect|AssignTagSetbyCallerMagnitude (GameplayEffects|MakeOutgoingSpec :self (Variables|Default|GetWeaverAbilitySystemComponent) :GameplayEffectClass "/Game/Shared/GameplayEffects/GE_Shared_ChangeAttackMultiplier.GE_Shared_ChangeAttackMultiplier_C" :Level 1.0) "(TagName=\"Shared.SetByCaller.AttackMultiplier\")" (Math|Conversions|ToFloat(Integer) (Variables|Attributes|GetFocusAttackMultiplier) 1.0)))
      (GameplayEffects|ApplyGameplayEffectSpecToSelf (Variables|Default|GetWeaverAbilitySystemComponent) _returnvalue))
    (:then_1
      (Class|PlayerCombatComponent|AddandSetElement (Variables|Default|GetPlayerCombatComponent) "/Game/Shared/Affixes/Elements/DataAssets/DA_Element_Arcane.DA_Element_Arcane"))
    (:then_2
      (Class|PlayerCombatComponent|AddandSetEffect (Variables|Default|GetPlayerCombatComponent) "/Game/Shared/Affixes/Effects/DataAssets/DA_Effect_Empty.DA_Effect_Empty"))))

(fn ConstructionScript)