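; Sevarog enemy character that selects its slash combat element on BeginPlay and can flag incoming projectiles for dodging.
; A camera shake gameplay event plays the Sevarog recall shake on the player stored as the blackboard's TargetActor.
; When a projectile enters the threat detection box, a line trace along its velocity adds the CanDodge tag if it would hit Sevarog.
; The node enabling that box's collision is disconnected.
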(event EventBeginPlay
  (|CallParentFunction)
  (Utilities|FlowControl|Sequence
    (:then_0
      (Class|EnemyCombatComponent|SetSelectedElement (Variables|Default|GetEnemyCombatComponent) "/Game/Shared/Affixes/Elements/DataAssets/DA_Element_SevarogSlash.DA_Element_SevarogSlash"))
    (:then_1
      (Ability|Async|WaitGameplayEventToActor 0 "(TagName=\"Shared.Event.CameraShake\")"
        (:EventReceived
          (bind _asweaver_player_character (Utilities|Casting|CastToWeaverPlayerCharacter (AI|Components|Blackboard|GetValueasObject (AI|GetBlackboard 0) (Utilities|Name|MakeLiteralName "TargetActor"))))
          (bind _asplayer_controller (Utilities|Casting|CastToPlayerController (Pawn|GetController _asweaver_player_character)))
          (Game|Feedback|ClientStartCameraShake _asplayer_controller "/Game/Characters/EnemyCharacters/Sevarog/CameraShake_SevarogRecall.CameraShake_SevarogRecall_C" 1.0 "CameraLocal" "0, 0, 0"))))))

(event EventOnThreatDetectionCollisionBoxBeginOverlap
  (params (OverlappedComponent :type Primitive%20Component%20Object%20Reference) (OtherActor :type Actor%20Object%20Reference) (OtherComp :type Primitive%20Component%20Object%20Reference) (OtherBodyIndex :type Integer) (bFromSweep :type Boolean) (SweepResult :type Hit%20Result%20Structure%20%28by%20ref%29))
  (bind _returnvalue (Transformation|GetActorLocation OtherActor))
  (bind _asweaver_projectile_base (Utilities|Casting|CastToWeaverProjectileBase OtherActor))
  (bind _outhits (Class|KismetSystemLibrary|LineTraceMultiforObjects _returnvalue (+ (* (Math|Vector|Normalize (Variables|/Script/Engine.MovementComponent|GetVelocity (Variables|/Script/Weaver.WeaverProjectileBase|GetProjectileMovementComp _asweaver_projectile_base))) 1e+03) _returnvalue) (Variables|Default|GetObject%20Types) false 0 "None" false))
  (bind _array_element (Utilities|Array|ForEachLoopwithBreak _outhits :!label _label)
    (:LoopBody
      (if (== (.HitActor (Collision|BreakHitResult _array_element)) self)
        (Class|WeaverFunctionLibrary|AddGameplayTagtoActorifNone self "(TagName=\"Shared.Status.CanDodge\")")
        (goto _label Break)))))

(fn ConstructionScript
  (|CallParentFunction))