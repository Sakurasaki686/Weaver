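; Base Blueprint for enemy characters, handling what happens when an enemy dies.
; On OnEnemyDied it disables capsule collision, then plays a Dissolve timeline that drives the mesh materials' DissolveAmount parameter and destroys the actor when finished.
; As the dissolve starts, a weighted random roll on AetherSpawnedChance can spawn a BP_Aether at the enemy's transform, with the enemy as instigator.
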(event EventBeginPlay)

(event Collision|EventActorBeginOverlap
  (params (OtherActor :type Actor%20Object%20Reference)))

(event EventTick
  (params (DeltaSeconds :type Float%20%28single-precision%29)))

(event EventOnEnemyDied
  (Utilities|FlowControl|Sequence
    (:then_0
      (Collision|SetCollisionEnabled (Variables|Default|GetCapsuleComponent) "NoCollision"))
    (:then_1
      (bind _dissolveamount (Timeline|Dissolve PlayFromStart)
        (:Update
          (Rendering|Material|SetScalarParameterValueonMaterials (Variables|Character|GetMesh) "DissolveAmount" _dissolveamount))
        (:Finished
          (Actor|DestroyActor))))
    (:then_2
      (if (Math|Random|RandomBoolwithWeight (Variables|Combat|GetAetherSpawnedChance))
        (Game|SpawnActorfromClass "/Game/Shared/BP_Aether.BP_Aether_C" (Math|Transform|MakeTransform (Transformation|GetActorLocation) (Transformation|GetActorRotation) "1.000000,1.000000,1.000000") "AdjustIfPossibleButAlwaysSpawn" "MultiplyWithRoot" 0 self)))))

(fn ConstructionScript)