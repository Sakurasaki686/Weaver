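; Earth shrine actor that the player activates with F after overlapping its activation range, which enables input.
; Activation spawns a circle particle, shakes the camera to fake an earthquake and plays a rumble sound.
; A timeline drives shrine emissive, animation play rate, light intensity and particle visibility through dynamic material instances and component setters.
; The timeline also disables input once activation starts; leaving the range does not.
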(event OnComponentBeginOverlap(Activation_Range)
  (params (OverlappedComponent :type Primitive%20Component%20Object%20Reference) (OtherActor :type Actor%20Object%20Reference) (OtherComp :type Primitive%20Component%20Object%20Reference) (OtherBodyIndex :type Integer) (bFromSweep :type Boolean) (SweepResult :type Hit%20Result%20Structure%20%28by%20ref%29))
  ;[1 1 1] Activate Shrine only possible Inside the Box Collsion
  (Input|EnableInput (Game|GetPlayerController 0))
  ;[1 1 1] Increase Emissive Intensity with use of Material Multipy Parameter
  (bind _returnvalue (Rendering|Material|CreateDynamicMaterialInstance (Variables|Default|GetShrine_Earth) 0 "/Game/MagicShrines/Materials/M_Shrine_Earth.M_Shrine_Earth" "None" :!class /Script/Engine.PrimitiveComponent)))

(event Input|KeyboardEvents|F
  (params (Key :type Key%20Structure :default "None"))
  ;[1 1 1] F to activate Shrine
  (:Pressed
    (Utilities|FlowControl|Sequence
      (:then_0
        ;[1 1 1] Spawn Circle Particle at Shrine Location with Z-Offset
        (bind _returnvalue (Effects|SpawnEmitteratLocation "/Game/MagicShrines/Particles/P_Circle_Earth.P_Circle_Earth" (+ (Transformation|GetWorldLocation (Variables|Default|GetShrine_Earth)) "0, 0,45.000000")))
        ;[1 1 1] Blend Circle Particle In/Out by the use of Material Visibility Parameter
        (bind _returnvalue_2 (Rendering|Material|CreateDynamicMaterialInstance _returnvalue 0 "/Game/MagicShrines/Materials/M_Circle.M_Circle" "None" :!class /Script/Engine.PrimitiveComponent))
        (bind _returnvalue_3 (Rendering|Material|CreateDynamicMaterialInstance _returnvalue 1 "/Game/MagicShrines/Materials/M_Ring.M_Ring" "None" :!class /Script/Engine.PrimitiveComponent))
        (bind _returnvalue_4 (Rendering|Material|CreateDynamicMaterialInstance _returnvalue 2 "/Game/MagicShrines/Materials/M_Dot.M_Dot" "None" :!class /Script/Engine.PrimitiveComponent)))
      (:then_1
        ;[1 1 1] Blend Particle In/Out with use of Material Visibility Parameter
        (bind _returnvalue_5 (Rendering|Material|CreateDynamicMaterialInstance (Variables|Default|GetFireflys) 0 0 "None" :!class /Script/Engine.PrimitiveComponent)))
      (:then_2
        ;[1 1 1] Timeline to adjust Emissive Intensity, Animation Play Rate etc.
        (bind (_direction _emissive _animation _light _spawn_particle _particle) (Timeline|Timeline_0 PlayFromStart)
          (:Update
            (Utilities|FlowControl|Sequence
              (:then_0
                ;[1 1 1] Increase Emissive Intensity with use of Material Multipy Parameter
                (Rendering|Material|SetScalarParameterValue (stale OnComponentBeginOverlap(Activation_Range) _returnvalue) "Emissive_Intensity" _emissive :!class /Script/Engine.MaterialInstanceDynamic))
              (:then_1
                ;[1 1 1] Animation Play Rate
                (Components|Timeline|SetPlayRate (Variables|Default|GetShrine_Earth) _animation))
              (:then_2
                ;[1 1 1] Shrine Light Intensity
                (Rendering|Components|Light|SetIntensity (Variables|Default|GetShrineLight) _light))
              (:then_3
                (Rendering|Material|SetScalarParameterValue _returnvalue_4 "Visibility" _spawn_particle :!class /Script/Engine.MaterialInstanceDynamic))
              (:then_4
                (Rendering|Material|SetScalarParameterValue _returnvalue_5 "Visibility" _particle :!class /Script/Engine.MaterialInstanceDynamic))
              (:then_5
                ;[1 1 1] Disable Player Input after Shrine Activation
                (Input|DisableInput (Game|GetPlayerController 0)))))))
      (:then_3
        ;[1 1 1] World Camera Shake to fake Earthquake
        (Camera|PlayWorldCameraShake "/Game/MagicShrines/Blueprints/BP_Camera_Shake.BP_Camera_Shake_C" (Transformation|GetActorLocation) 0.0 1e+03))
      (:then_4
        ;[1 1 1] Rumble Sound after Activation
        (Audio|PlaySoundatLocation "/Game/MagicShrines/Audio/SC_Rumble.SC_Rumble" (Transformation|GetWorldLocation (Variables|Default|GetShrine_Earth)) "0, 0, 0" 4.0 1.0 0.0 0 0 0 0)))))

(fn ConstructionScript)