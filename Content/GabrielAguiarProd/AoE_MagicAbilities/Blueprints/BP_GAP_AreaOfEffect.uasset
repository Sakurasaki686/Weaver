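; BP_GAP_AreaOfEffect is a configurable actor that displays an area-of-effect particle effect and destroys itself after a set delay.
; The construction script assigns the chosen particle template, optionally overrides its Color parameter, and passes Scale as both a vector and an X-only float parameter.
; BeginPlay reassigns the template, offsets the actor by Location, sets its Rotation, then starts the destroy timer.
; It contains no active overlap, damage or tick logic.
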(event Custom|SpawnAoE
  (Effects|Components|ParticleSystem|SetTemplate (Variables|Default|GetAreaOfEffect) (Variables|Default|GetVFXAreaOfEffect))
  (Transformation|SetActorLocationAndRotation (+ (Transformation|GetActorLocation) (Variables|Default|GetLocation)) (Variables|Default|GetRotation)))

(event EventBeginPlay
  (CallFunction|SpawnAoE)
  (Utilities|FlowControl|Delay (Variables|Default|GetDelayBeforeDestroying))
  (Actor|DestroyActor))

(event Collision|EventActorBeginOverlap
  (params (OtherActor :type Actor%20Object%20Reference)))

(event EventTick
  (params (DeltaSeconds :type Float%20%28single-precision%29)))

(fn ConstructionScript
  (bind _areaofeffect (Variables|Default|GetAreaOfEffect))
  (bind _scale (Variables|Default|GetScale))
  (Effects|Components|ParticleSystem|SetTemplate (Variables|Default|GetAreaOfEffect) (Variables|Default|GetVFXAreaOfEffect))
  (if (Variables|Default|GetChangeColor%20?)
    (Effects|Components|ParticleSystem|SetColorParameter (Variables|Default|GetAreaOfEffect) "Color" (Variables|Default|GetColor)))
  (Effects|Components|ParticleSystem|SetVectorParameter _areaofeffect "Scale" _scale)
  (Effects|Components|ParticleSystem|SetFloatParameter _areaofeffect "Scale" (.X (Math|Vector|BreakVector _scale))))